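; BP_StageLocation is a stage location marker actor identified by a location number and ID.
; Its construction script writes both values to text components as labels.
; On BeginPlay it sets the static mesh's visibility from IsVisible, propagating the change to child components.
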(event `self.ReceiveBeginPlay`
  (`SceneComponent.SetVisibility` (`self.StaticMeshComponent`) (`self.IsVisible`) true))

(fn `UserConstructionScript`
  (`TextRenderComponent.K2_SetText` (`self.Text_LocationNumber`) (`KismetTextLibrary.Conv_NameToText` (`self.LocationNumber`)))
  (`TextRenderComponent.K2_SetText` (`self.Text_LocationId`) (`KismetTextLibrary.Conv_NameToText` (`self.LocationId`))))