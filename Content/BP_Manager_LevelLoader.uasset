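; Level loader manager actor that spawns instances of streaming levels at the transforms of designated location actors.
; LoadLevels runs on BeginPlay when enabled and set to auto-load, after validating that the name and location arrays match and are not empty.
; Each streaming level gets a uniquely named instance via CreateInstance and an incrementing ID, set to block on load and be visible.
; It stores the instances, then calls AllLevelsAreLoaded and flags loading as done.
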(event `self.ReceiveBeginPlay`
  (`|ExecutionSequence`
    (:`then_0`
      (`SceneComponent.SetVisibility` (`self.TextRender`) false false))
    (:`then_1`
      ;[1 1 1] Load Level if AutoLoad is set, dont enable if loading from another location
      (if (`self.AutoLoadLevels`)
        (if (`self.IsEnabled`)
          (`self.LoadLevels`))))))

(event `LoadLevels`
  (bind _levelnames (`self.LevelNames`))
  (if (`self.IsEnabled`)
    ;[1 1 1] Array Error Checks
    (bind _returnvalue (`self.CheckLevelNamesLocationsAreEqual`))
    (if _returnvalue
      (`|ExecutionSequence`
        (:`then_0`
          ;[1 1 1] Load Level
          (for (_array_element _array_index) _levelnames
            (bind _returnvalue_2 (`GameplayStatics.GetStreamingLevel` _array_element))
            (if (!= _returnvalue_2 null)
              (`|ExecutionSequence`
                (:`then_0`
                  (bind _returnvalue_3 (`LevelStreaming.CreateInstance` _returnvalue_2 (`KismetStringLibrary.Concat_StrStr` (`KismetStringLibrary.Conv_NameToString` (`|GetArrayItem` _levelnames _array_index)) (`KismetStringLibrary.Concat_StrStr` "_" (`KismetStringLibrary.Conv_IntToString` (`self.UniqueLevelID`))))))
                  (set `LevelStreaming.LevelTransform` (`|GetArrayItem` (`/VideoCore/Blueprints/BP_VideoCoreFunctionLibrary.Get Actor Transforms Array` (`self.LevelLocations`)) _array_index) _returnvalue_3)
                  (set `LevelStreaming.bShouldBeLoaded` true _returnvalue_3)
                  (set `LevelStreaming.bShouldBlockOnLoad` true _returnvalue_3)
                  (set `LevelStreaming.bShouldBeVisible` true _returnvalue_3)
                  (`KismetArrayLibrary.Array_Add` (`self.LoadedStreamedLevels`) _returnvalue_3))
                (:`then_1`
                  (bind _result (`/Engine/EditorBlueprintResources/StandardMacros.IncrementInt` (`self.UniqueLevelID`))
                    (:`  `
                      (set `self.UniqueLevelID` _result))))))))
        (:`then_1`
          (`self.AllLevelsAreLoaded`)
          (set `self.LevelsLoaded` true))))))

(fn `CheckLevelNamesLocationsAreEqual`
  (returns (ReturnValue :type Boolean))
  (locals (IsTrue :type Boolean))
  (bind _returnvalue (`KismetArrayLibrary.Array_Length` (`self.LevelNames`)))
  (bind _returnvalue_2 (`KismetArrayLibrary.Array_Length` (`self.LevelLocations`)))
  (if (== _returnvalue _returnvalue_2)
    (if (!= _returnvalue 0)
      (if (!= _returnvalue_2 0)
        (set `local.IsTrue` true)
        (`KismetSystemLibrary.PrintString` "Level Loader: Levels Loading" true true (struct :`R` 1.0 :`G` 0.672443 :`A` 1.0))
        (else
          (`KismetSystemLibrary.PrintString` "Level Loader: No Level Locations Set" true true (struct :`R` 1.0 :`G` 0.672443 :`A` 1.0))))
      (else
        (`KismetSystemLibrary.PrintString` "Level Loader: No Level Names Set" true true (struct :`R` 1.0 :`G` 0.672443 :`A` 1.0))))
    (else
      (`KismetSystemLibrary.PrintString` "Level Loader: Leve location amount mismatch" true true (struct :`R` 1.0 :`G` 0.672443 :`A` 1.0))))
  (return (`local.IsTrue`)))

(fn `UserConstructionScript`)