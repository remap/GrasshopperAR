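; Placeable god ray effect that combines a light-shaft card mesh, optional dust particles and an optional spotlight.
; The construction script does all the work, pushing exposed settings into a dynamic card material, with an experimental convergent-ray variant.
; Length and diameter multipliers drive card scale, smoke tiling and panning, dust bounds and spawn amount, and spotlight radius and cone angle.
; The event graph is empty, so nothing updates at runtime from this Blueprint.
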(fn `UserConstructionScript`
  (locals (godray_card_MI :type "MaterialInstance Object Reference" :default "MaterialInstanceConstant'/Game/lazygodray/lazygodray_components/godray_card_MI.godray_card_MI'") (godray_card_MI_convergent :type "MaterialInstance Object Reference" :default "MaterialInstanceConstant'/Game/lazygodray/lazygodray_components/godray_card_MI_convergent.godray_card_MI_convergent'") (godray_mtl_dynamic_instance :type "MaterialInstanceDynamic Object Reference") (dust_mtl_dynamic_instance :type "MaterialInstanceDynamic Object Reference") (godray_dust :type "ParticleSystemComponent Object Reference") (godray_dust_parameters :type "Array of ParticleSysParam Structure") (godray_dust_MI :type "MaterialInstance Object Reference" :default "MaterialInstanceConstant'/Game/lazygodray/lazygodray_components/godray_dust_MI.godray_dust_MI'"))
  (bind _godray_card_sm (`self.godray_card_SM`))
  (bind _length_multiplier (`self.length multiplier`))
  (bind _godray_card_sm_2 (`self.godray_card_SM`))
  (bind _size_multiplier (`self.size multiplier`))
  (bind _godray_dust (`local.godray_dust`))
  (bind _ps_bounds (`self.PS Bounds`))
  (bind _diameter_multiplier (`self.diameter multiplier`))
  (bind _godray_dust_2 (`local.godray_dust`))
  (bind _spotlight (`self.SpotLight`))
  (bind _smoke_texture_scale (`self.smoke texture scale`))
  (bind _returnvalue (* (`self.velocity multiplier`) 0.5))
  (bind _returnvalue_2 (* (* (`self.diameter multiplier`) 40.0) (`self.spawn radius multiplier`)))
  (`self.SetActorScale3D` (1.0 1.0 1.0))
  ;[1 1 1] lightray convergent experimental feature
  (if (`self.use lightray convergent`)
    (bind _returnvalue_3 (`PrimitiveComponent.CreateDynamicMaterialInstance` _godray_card_sm 0 (`local.godray_card_MI_convergent`) "None"))
    (set `local.godray_mtl_dynamic_instance` _returnvalue_3)
    (`MeshComponent.SetScalarParameterValueOnMaterials` (`self.godray_card_SM`) "lightray convergent" (`self.lightray convergent rate`))
    (else
      (bind _returnvalue_4 (`PrimitiveComponent.CreateDynamicMaterialInstance` _godray_card_sm 0 (`local.godray_card_MI`) "None"))
      (set `local.godray_mtl_dynamic_instance` _returnvalue_4)))
  ;[1 1 1] godray card material parameters
  (`SceneComponent.SetRelativeScale3D` (`self.godray_card_SM`) (`KismetMathLibrary.MakeVector` (`self.length multiplier`) _diameter_multiplier _diameter_multiplier))
  (`MeshComponent.SetScalarParameterValueOnMaterials` _godray_card_sm_2 "overall intensity" (`self.overall intensity`))
  (`MeshComponent.SetVectorParameterValueOnMaterials` _godray_card_sm_2 "tint color" (`KismetMathLibrary.Conv_LinearColorToVector` (`self.tint color`)))
  (`MeshComponent.SetScalarParameterValueOnMaterials` _godray_card_sm_2 "overall contrast" (`self.overall contrast`))
  (`MaterialInstanceDynamic.SetTextureParameterValue` (`local.godray_mtl_dynamic_instance`) "lightshaft texture" (`self.light shaft texture`))
  (`MeshComponent.SetScalarParameterValueOnMaterials` _godray_card_sm_2 "streak strength" (`self.light shaft strength`))
  (`MeshComponent.SetScalarParameterValueOnMaterials` _godray_card_sm_2 "streaks amount multiplier" (`self.light shaft amount`))
  (`MeshComponent.SetScalarParameterValueOnMaterials` _godray_card_sm_2 "streaks length multiplier" (`self.light shaft length`))
  (`MeshComponent.SetScalarParameterValueOnMaterials` _godray_card_sm_2 "depth fade" (`self.depth fade distance`))
  (`MeshComponent.SetScalarParameterValueOnMaterials` _godray_card_sm_2 "fresnel exponent" (`self.fesnel exponent`))
  (`MeshComponent.SetScalarParameterValueOnMaterials` _godray_card_sm_2 "fading starting distance" (`self.camera fading starting distance`))
  (`MeshComponent.SetScalarParameterValueOnMaterials` _godray_card_sm_2 "fading transition range" (`self.camera fading transition range`))
  (`MeshComponent.SetScalarParameterValueOnMaterials` _godray_card_sm_2 "falloff midpoint" (`self.vertical falloff midpoint`))
  (`MeshComponent.SetScalarParameterValueOnMaterials` _godray_card_sm_2 "falloff exponent" (`self.vertical falloff exponent`))
  (`MeshComponent.SetScalarParameterValueOnMaterials` _godray_card_sm_2 "cylindrical falloff exponent" (`self.cylindrical masking exponent`))
  (`MeshComponent.SetScalarParameterValueOnMaterials` _godray_card_sm_2 "falloff strength" (`self.vertical falloff strength`))
  (`MaterialInstanceDynamic.SetTextureParameterValue` (`local.godray_mtl_dynamic_instance`) "masking texture" (`self.smoke texture`))
  (`MeshComponent.SetScalarParameterValueOnMaterials` _godray_card_sm_2 "detail intensity" (`self.smoke intensity`))
  (`MeshComponent.SetScalarParameterValueOnMaterials` _godray_card_sm_2 "detail texture tilingX" (* _smoke_texture_scale (`self.diameter multiplier`)))
  (`MeshComponent.SetScalarParameterValueOnMaterials` _godray_card_sm_2 "detail texture tilingY" (* _smoke_texture_scale (`self.length multiplier`)))
  (`MeshComponent.SetScalarParameterValueOnMaterials` _godray_card_sm_2 "detail Xspeed" (/ (`self.panning speedX`) (`self.diameter multiplier`)))
  (`MeshComponent.SetScalarParameterValueOnMaterials` _godray_card_sm_2 "detail Yspeed" (/ (`self.panning speedY`) (`self.length multiplier`)))
  (if (`self.enable dust particle. cannot be toggled during runtime.`)
    ;[1 1 1] particle system parameters
    (`BoxComponent.SetBoxExtent` _ps_bounds (`KismetMathLibrary.MakeVector` (* (* (`self.length multiplier`) 50.0) (`self.spawn length multiplier`)) _returnvalue_2 _returnvalue_2) false)
    (bind _returnvalue_5 (`AddComponent|NODE_AddParticleSystemComponent-0`))
    (bind _output_get (set `local.godray_dust` _returnvalue_5))
    (set `SceneComponent.bUseAttachParentBound` true _output_get)
    (`SceneComponent.K2_AttachToComponent` _output_get _ps_bounds "None" "KeepRelative" "KeepRelative" "KeepRelative" false)
    (bind _returnvalue_6 (`PrimitiveComponent.CreateDynamicMaterialInstance` _output_get 0 (`local.godray_dust_MI`) "None"))
    (set `local.dust_mtl_dynamic_instance` _returnvalue_6)
    (bind _output_get_2 (set `local.godray_dust_parameters` (`ParticleSystemComponent.InstanceParameters` _godray_dust)))
    (`KismetArrayLibrary.Array_Add` _output_get_2 (make `ParticleSysParam` "size" "PSPT_VectorRand" 0.0 0.0 (`KismetMathLibrary.Conv_DoubleToVector` _size_multiplier) (`KismetMathLibrary.Conv_DoubleToVector` (* (/ (`self.size minimum percentage`) 100.0) _size_multiplier))))
    (`KismetArrayLibrary.Array_Add` _output_get_2 (make `ParticleSysParam` "V" "PSPT_VectorRand" 0.0 0.0 (`KismetMathLibrary.Conv_DoubleToVector` (+ _returnvalue 0.5)) (`KismetMathLibrary.Conv_DoubleToVector` (- 0.5 _returnvalue))))
    (set `ParticleSystemComponent.InstanceParameters` _output_get_2 _godray_dust)
    (`SceneComponent.K2_SetRelativeLocation` _ps_bounds (`KismetMathLibrary.MakeVector` (* (+ (* _length_multiplier 0.5) (* _length_multiplier (* (`self.spawn location vertical offset`) -1.0))) 100.0)) false false)
    (`ParticleSystemComponent.SetVectorParameter` _godray_dust_2 "dust color" (`KismetMathLibrary.Conv_LinearColorToVector` (`self.particle color`)))
    (`ParticleSystemComponent.SetFloatParameter` _godray_dust_2 "cylinderHeight" (* (* (`self.length multiplier`) 100.0) (`self.spawn length multiplier`)))
    (`ParticleSystemComponent.SetFloatParameter` _godray_dust_2 "cylinderRadius" (* (* (`self.diameter multiplier`) 40.0) (`self.spawn radius multiplier`)))
    (`ParticleSystemComponent.SetFloatParameter` _godray_dust_2 "spawn" (* (* (`self.amount multiplier`) (`self.diameter multiplier`)) (`self.length multiplier`)))
    (`ParticleSystemComponent.SetFloatParameter` _godray_dust_2 "revealing distance" (`self.revealing distance`))
    (`ParticleSystemComponent.SetFloatParameter` _godray_dust_2 "revealing transition" (`self.revealing transition`))
    (`ParticleSystemComponent.SetFloatParameter` _godray_dust_2 "culling distance" (`self.culling distance`))
    (`ParticleSystemComponent.SetFloatParameter` _godray_dust_2 "culling transition" (`self.culling transition`)))
  ;[1 1 1] spotlight parameters
  (`SceneComponent.SetVisibility` _spotlight (`self.enable spotlight component; cannot be toggled during runtime`) false)
  (`PointLightComponent.SetAttenuationRadius` _spotlight (+ (* (`self.length multiplier`) 100.0) (* (`self.attenuation offset`) (`self.diameter multiplier`))))
  (`SpotLightComponent.SetOuterConeAngle` _spotlight (+ (`KismetMathLibrary.DegAtan` (/ (/ (`self.diameter multiplier`) 2.0) (`self.length multiplier`))) (`self.outer cone angle offset`)))
  (`LightComponent.SetLightColor` _spotlight (`self.tint color`) true)
  (`LightComponent.SetIntensity` _spotlight (`self.light intensity in Lumens`))
  (`SpotLightComponent.SetInnerConeAngle` _spotlight (`self.inner cone angle`))
  (`PointLightComponent.SetSourceRadius` _spotlight (* (`self.light source radius`) (`self.diameter multiplier`))))