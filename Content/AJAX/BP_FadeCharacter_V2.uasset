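; BP_FadeCharacter_V2 plays a video character on a plane, using a separate alpha video alongside the colour video.
; On BeginPlay it creates a dynamic M_ChromaKey1 material, binds both media textures to their players, then opens and plays both sources.
; An optional horizontal flip swaps the material's u1 and u2 parameters.
; Despite the name, no fade runs here, as the Dissolve parameter setter is never called.
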(event `self.ReceiveBeginPlay`
  (bind _mediatex (`self.MediaTex`))
  (bind _mediaplayer (`self.MediaPlayer`))
  (bind _mediaplayer_alpha (`self.MediaPlayer_Alpha`))
  (bind _mediatex_alpha (`self.MediaTex_Alpha`))
  (`|ExecutionSequence`
    (:`then_0`
      (bind _returnvalue (`PrimitiveComponent.CreateDynamicMaterialInstance` (`self.Plane`) 0 "/Game/AJAX/M_ChromaKey1.M_ChromaKey1" "None"))
      (bind _output_get (set `self.Material_Instance` _returnvalue))
      (`/Engine/EditorBlueprintResources/StandardMacros.IsValid` _mediatex
        (:`Is Valid`
          (`/Engine/EditorBlueprintResources/StandardMacros.IsValid` _mediatex_alpha
            (:`Is Valid`
              (`MaterialInstanceDynamic.SetTextureParameterValue` _output_get "Video" _mediatex)
              (`MaterialInstanceDynamic.SetTextureParameterValue` _output_get "Video_Alpha" _mediatex_alpha)
              (`MediaTexture.SetMediaPlayer` _mediatex (`self.MediaPlayer`))
              (`MediaTexture.SetMediaPlayer` _mediatex_alpha (`self.MediaPlayer_Alpha`))
              (if (`self.Flip Horizontal`)
                (`self.Flip Texture Horizontal`)))))))
    (:`then_1`
      (`MediaPlayer.OpenSource` _mediaplayer (`self.FileMediaSource`))
      (`MediaPlayer.Play` _mediaplayer))
    (:`then_2`
      (`MediaPlayer.OpenSource` _mediaplayer_alpha (`self.FileMediaSource_Alpha`))
      (`MediaPlayer.Play` _mediaplayer_alpha))))

(fn `Flip Texture Horizontal`
  (bind _material_instance (`self.Material_Instance`))
  (bind _isa (`/Engine/EditorBlueprintResources/StandardMacros.FlipFlop`)
    (:`A`
      _)
    (:`B`
      _))
  (bind _returnvalue (`KismetMathLibrary.SelectFloat` 1.0 0.0 _isa))
  (`MaterialInstanceDynamic.SetScalarParameterValue` _material_instance "u1" _returnvalue)
  (`MaterialInstanceDynamic.SetScalarParameterValue` _material_instance "u2" (- 1.0 _returnvalue)))

(fn `UserConstructionScript`)