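; Instancing actor that scatters copies of a mesh, yellow bellflowers going by the asset name, inside a small box.
; The construction script loops up to ObjectCount, adding Instanced Static Mesh instances at random points with a fixed rotation and unit scale.
; Each pass also prints a debug point, re-rolled separately so it differs from the placed location.
; The event graph holds only disabled stubs.
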(fn `UserConstructionScript`
  (bind _returnvalue (`KismetMathLibrary.RandomPointInBoundingBox` (0.0 0.0 40.0) (50.0 40.0 60.0)))
  (for _index (range 1 (+ (`self.Object Count`) 1))
    (`InstancedStaticMeshComponent.AddInstance` (`self.InstancedStaticMesh`) (`KismetMathLibrary.MakeTransform` _returnvalue (struct :`Yaw` 90.0 :`Roll` 180.0)))
    (`KismetSystemLibrary.PrintString` (`KismetStringLibrary.Conv_VectorToString` _returnvalue) true true (struct :`G` 0.66 :`B` 1.0 :`A` 1.0) 10.0)))