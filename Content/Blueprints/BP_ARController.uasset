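; AR player controller that starts the AR session on capable devices, restores player name and auto-reconnects to the server; the VR branch is empty.
; Fiducial anchors from BPRelocalizer, optionally confirmed by popup, set alignment and have the GameInstance stream that anchor's levels and move the player there.
; Limbo events exit the game level back to the player start.
; Multitouch holds toggle the master debug UI or temporarily unload AR-prefixed sublevels.
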(event `self.ReceiveBeginPlay`
  (bind _returnvalue (`blueprintHelpers.isArCapableDevice`))
  (if _returnvalue
    (`self.On BeginPlay AR`)
    (else
      (`self.On BeginPlay VR`))))

(event `On BeginPlay VR`)

(event `On BeginPlay AR`
  (bind _game_instance (`/Game/Blueprints/BP_GhLibrary.Get My Game Instance`))
  (bind _bp_relocalizer (`self.BP_Relocalizer`))
  (bind _bp_augmenteddebugger (`self.BP_AugmentedDebugger`))
  (bind (_additionalinfo _status) (break `ARSessionStatus` (`ARBlueprintLibrary.GetARSessionStatus`)))
  (bind _playername (`/Game/Blueprints/BP_GHSaveGame.playerName` (`/Game/Blueprints/BP_GameInstance.saveGame` (`/Game/Blueprints/BP_GhLibrary.Get My Game Instance`))))
  (`|ExecutionSequence`
    (:`then_0`
      (`/Game/Blueprints/BP_GameInstance.Set HUD Visibility` (`/Game/Blueprints/BP_GhLibrary.Get My Game Instance`) true)
      ;[0.04036 0.3879 1] AR Device UI Control Setup
      (add `self.OnToggleMasterUiDelegate` (delegate `On Toggle Master UI`)))
    (:`then_1`
      ;[0.2862 0.1947 1] AR Session Setup
      (switch `EARSessionStatus` _status
        (:`NotStarted`
          (`DDBlueprintLibrary.LogDebug` "Starting AR Session")
          (if (`/DDAugmented/BP_AugmentedDebugger.isDebugSession` (`self.BP_AugmentedDebugger`)) :!label _label
            (`/DDAugmented/BP_AugmentedDebugger.Init Debubg Session` _bp_augmenteddebugger)
            (`DDBlueprintLibrary.LogDebug` "Loaded debug AR session")
            (else
              (`/DDAugmented/BP_AugmentedDebugger.Init Release Session` _bp_augmenteddebugger "/Game/Data/D_SessionConfig_211110.D_SessionConfig_211110" :!label _label_2)
              (`DDBlueprintLibrary.LogDebug` "Loaded release AR session")))
          (add `/DDAugmented/BP_AugmentedDebugger.On AR Session Started` _bp_augmenteddebugger (delegate `On AR Session Started`)))
        (:`Running`
          (`ARBlueprintLibrary.StopARSession`)
          (goto _label))
        (:`NotSupported`
          (`DDBlueprintLibrary.LogWarning` (`KismetTextLibrary.Conv_TextToString` (`|FormatText` "Unsupported AR Session status {status}" (`KismetTextLibrary.Conv_ByteToText` _status))) :!label _label_3))
        (:`FatalError`
          (goto _label_3))
        (:`PermissionNotGranted`
          (goto _label_3))
        (:`UnsupportedConfiguration`
          (goto _label_3))
        (:`Other`
          (goto _label_3))))
    (:`then_2`
      ;[0.261 1 0.3132] Fiducial-Based Relocalization
      (`GameplayStatics.UnloadStreamLevel` "M_Lobby")
      (add `FiducialRelocalizerComponent.OnNewPawnEstimation` _bp_relocalizer (delegate `On Fiducial Anchored`))
      (add `FiducialRelocalizerComponent.OnGoBackToLimbo` _bp_relocalizer (delegate `On Must Go To Limbo`)))
    (:`then_3`
      (`|ExecutionSequence`
        (:`then_0`
          ;[1 1 1] server connection status handling
          (`|ExecutionSequence`
            (:`then_0`
              (add `GHGameInstance.OnConnectionStatusUpdated` _game_instance (delegate `On Connection Status Updated`)))
            (:`then_1`
              (if (`/Game/Blueprints/BP_GHSaveGame.autoReconnect` (`/Game/Blueprints/BP_GameInstance.saveGame` _game_instance)) :!label _label_4
                (`/Game/Blueprints/BP_GameInstance.Handle Server Reconnect` _game_instance "Disconnected" (`GHGameInstance.getConnectionStatus` _game_instance))))))
        (:`then_1`
          ;[1 1 1] because... unreal
          (`KismetSystemLibrary.Delay` 2.0)
          ;[1 1 1] load player name
          (`/Engine/EditorBlueprintResources/StandardMacros.IsValid` (`self.PlayerState`)
            (:`Is Valid`
              (if (not (`KismetStringLibrary.IsEmpty` _playername))
                (`self.SetNewPlayerName` _playername)))
            (:`Is Not Valid`
              (`DDBlueprintLibrary.LogError` "Can't set player name"))))))))

(event `InputTouch`
  (params (Location :type "Vector Structure") (FingerIndex :type "ETouchIndex Enum"))
  ;[0.3245 0.6496 1] MASTER DEBUG UI. Multitouch-enabled
  (:`Pressed`
    (`self.Check Touch Is Valid` FingerIndex
      (:`valid`
        (`self.OnToggleMasterUiDelegate`))
      (:`Invalid`
        (`self.Check Touch Is Valid` FingerIndex "Touch2"
          (:`valid`
            (bind _ntoggled (`self.Toggle AR Sublevels`))))))))

(event `On Toggle Master UI`
  ;[0.04036 0.3879 1] AR Device UI Control Setup
  (`/Game/Blueprints/BP_GameInstance.Toggle Master UI` (`/Game/Blueprints/BP_GhLibrary.Get My Game Instance`) (`GameplayStatics.GetPlayerController` 0)))

(event `On InfoPopup Hide`
  (params (popupWidget :type "/Game/Blueprints/UI/BP_HUD_Popup Object Reference"))
  ;[0.3245 0.6496 1] MASTER DEBUG UI. Multitouch-enabled
  ;;[1 0.3905 0] visual notification (disabled)
  (if (> (`/Game/Blueprints/UI/BP_HUD_Popup.buttonPressed` popupWidget) 0)
    (set `self.temporaryArLevelsInfoPopup` false)))

(event `On AR Session Picked`
  (params (popupWidget :type "/Game/Blueprints/UI/BP_HUD_Popup Object Reference"))
  ;[0.2862 0.1947 1] AR Session Setup
  (if (> (`/Game/Blueprints/UI/BP_HUD_Popup.buttonPressed` popupWidget) 0)
    (`/Game/Blueprints/BP_GameInstance.Hide Popup` (`/Game/Blueprints/BP_GhLibrary.Get My Game Instance`))
    (goto _label)
    (else
      (goto _label_2))))

(event `On AR Session Started`
  ;[0.2862 0.1947 1] AR Session Setup
  (if (`GHPlayerState.isGameActive` (`/Game/Blueprints/BP_GhLibrary.Get My Player State`))
    (`/Game/Blueprints/BP_GameInstance.Exit Game Level` (`/Game/Blueprints/BP_GhLibrary.Get My Game Instance`) self)))

(event `self.exitGameLevel`
  ;[1 0.1728 0.7218] Called by GameInstance: Go back to player start in the loaded lobby levels (ARLimbo, VRLobby)
  (bind _playerstart (`/Game/Blueprints/BP_GhLibrary.Find Player Start` (`self.startTags`)))
  (bind _output_get (set `self.playerStart` _playerstart))
  (`/Game/Blueprints/BP_GhLibrary.Move Player To Start` self _output_get))

(event `On Must Go To Limbo`
  ;[0.261 1 0.3132] Fiducial-Based Relocalization
  ;;[1 0.0966 0.0966] Go To Limbo
  (`/Game/Blueprints/BP_GameInstance.Exit Game Level` (`/Game/Blueprints/BP_GhLibrary.Get My Game Instance`) self))

(event `self.enterGameLevel`
  (params (levels :type "Array of Name (by ref)"))
  (bind _returnvalue (`self.GetComponentByClass` "/DDAugmented/BP_AugmentedDebugger.BP_AugmentedDebugger_C"))
  ;[1 0.1135 0.8705] Called by GameInstance: Load all associated levels. Don't need to move pawn as it's already done
  (`/Game/Blueprints/BP_GhLibrary.Move Player To Start` self (`self.activeFanchor`) false)
  (`/Engine/EditorBlueprintResources/StandardMacros.IsValid` _returnvalue
    (:`Is Valid`
      (`AugmentedDebugger.ClientSetPawnAdjustment` _returnvalue (`AugmentedDebugger.GetPawnAdjustment` _returnvalue))
      (`AugmentedDebugger.ClientSetAlignmentAdjustment` _returnvalue (`AugmentedDebugger.GetAlignemntAdjustment` _returnvalue))
      (`/DDAugmented/BP_AugmentedDebugger.Server_ReportLoadedLevels` (`self.BP_AugmentedDebugger`) (`/Game/Blueprints/BP_GameInstance.Get Loaded Levels` (`/Game/Blueprints/BP_GhLibrary.Get My Game Instance`))))))

(event `On Fiducial Anchored`
  (params (fiducialName :type String) (arAlignment :type "Transform Structure") (fanchorTransform :type "Transform Structure") (fanchor :type "FAnchor Object Reference"))
  (bind _activefanchor (`self.activeFanchor`))
  ;[0.261 1 0.3132] Fiducial-Based Relocalization
  (set `self.activeFanchor` fanchor)
  (set `self.activeArAlignment` arAlignment)
  (if (`self.isShowingAnchoringPopup`)
    (`/Game/Blueprints/BP_GameInstance.Show Popup Custom` (`/Game/Blueprints/BP_GhLibrary.Get My Game Instance`) "Fiducial Relocalization" (`self.Relocalization Info Text` fanchor) 10 (`|MakeArray` "No" "Yes" "Yes, mute this") (delegate `On Relocalization Popup Hidden`))
    (else
      (`self.setArAlignment` (`self.activeArAlignment`) :!label _label_5)
      (`self.Debug Print Relocalization` (`FAnchor.FiducialName` _activefanchor) (`FAnchor.getAlignedTransform` _activefanchor))
      (`|ExecutionSequence`
        (:`then_0`
          (`/Game/Blueprints/BP_GameInstance.Enter Game Level` (`/Game/Blueprints/BP_GhLibrary.Get My Game Instance`) self (`FAnchor.StreamingLevels` _activefanchor) (`FAnchor.IsExclusive` _activefanchor)))
        (:`then_1`)))))

(event `On Relocalization Popup Hidden`
  (params (popupWidget :type "/Game/Blueprints/UI/BP_HUD_Popup Object Reference"))
  ;[0.261 1 0.3132] Fiducial-Based Relocalization
  (`/Game/Blueprints/BP_GameInstance.Hide Popup` (`/Game/Blueprints/BP_GhLibrary.Get My Game Instance`))
  (switch `int` (`/Game/Blueprints/UI/BP_HUD_Popup.buttonPressed` popupWidget)
    (:`Default`
      (goto _label_5))
    (:`1`
      (`/Game/Blueprints/BP_GameInstance.Show Popup` (`/Game/Blueprints/BP_GhLibrary.Get My Game Instance`) "Fiducial Ignored" "Relocalization skipped" 3))
    (:`2`
      (goto _label_5))
    (:`3`
      (set `self.isShowingAnchoringPopup` false)
      (goto _label_5))))

(event `On Connection Status Updated`
  (params (oldStatus :type "ConnectionStatus Enum" :default "Disconnected") (newStatus :type "ConnectionStatus Enum" :default "Disconnected"))
  ;[1 1 1] server connection status handling
  (goto _label_4))

(fn `Toggle AR Sublevels`
  (returns (nToggled :type Integer))
  (locals (nLevels :type Integer))
  (bind _game_instance (`/Game/Blueprints/BP_GhLibrary.Get My Game Instance`))
  (bind _temporaryhiddenlevels (`self.temporaryHiddenLevels`))
  (bind _temporaryhiddenlevels_2 (`self.temporaryHiddenLevels`))
  (if (`self.temporaryHidingArLevels`)
    (`/Game/Blueprints/BP_GameInstance.Stream Levels Synchronously` (`/Game/Blueprints/BP_GhLibrary.Get My Game Instance`) _temporaryhiddenlevels_2 false false)
    (set `local.nLevels` (`KismetArrayLibrary.Array_Length` _temporaryhiddenlevels_2))
    (`KismetArrayLibrary.Array_Clear` _temporaryhiddenlevels_2)
    (set `self.temporaryHidingArLevels` false)
    (`/DDAugmented/BP_AugmentedDebugger.Server_ReportLoadedLevels` (`self.BP_AugmentedDebugger`) (`/Game/Blueprints/BP_GameInstance.Get Loaded Levels` (`/Game/Blueprints/BP_GhLibrary.Get My Game Instance`)) :!label _label)
    (else
      (for _array_element (`/Game/Blueprints/BP_GameInstance.Filter Levels With Prefix` _game_instance (`/Game/Blueprints/BP_GameInstance.Get Loaded Levels` _game_instance) "AR_")
        (`KismetArrayLibrary.Array_Add` (`self.temporaryHiddenLevels`) _array_element))
      (if (> (`KismetArrayLibrary.Array_Length` (`self.temporaryHiddenLevels`)) 0)
        (`/Game/Blueprints/BP_GameInstance.Stream Levels Synchronously` (`/Game/Blueprints/BP_GhLibrary.Get My Game Instance`) _temporaryhiddenlevels true false)
        (set `local.nLevels` (`KismetArrayLibrary.Array_Length` _temporaryhiddenlevels))
        (set `self.temporaryHidingArLevels` true)
        (goto _label)
        (else
          _))))
  (return (`local.nLevels`)))

(fn `UserConstructionScript`
  (bind _playerstart (`/Game/Blueprints/BP_GhLibrary.Get Player Start With Tag` "ARStart"))
  (if (`KismetSystemLibrary.IsValid` _playerstart)
    (set `self.playerStart` _playerstart)
    (else
      (`DDBlueprintLibrary.LogError` "ARStart was not found. Fail over to VRStart")
      (bind _playerstart_2 (`/Game/Blueprints/BP_GhLibrary.Get Player Start With Tag` "VRStart"))
      (if (`KismetSystemLibrary.IsValid` _playerstart_2)
        (set `self.playerStart` _playerstart_2)
        (else
          (`DDBlueprintLibrary.LogError` "Fail-over VRStart was not found."))))))