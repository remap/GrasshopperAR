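; BP_Spectator is a multiplayer spectator pawn with a camera and a floating player name.
; On Tick, the autonomous proxy or authority sends location and camera rotation by server RPC into PawnTransform, whose OnRep moves the actor.
; Tick also applies that rotation to the camera and turns the name toward the first player controller.
; Name text is set once from Tick, as PlayerState is unavailable at BeginPlay.
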(event `RPC Server Pawn Transform Replicate`
  (params (transform :type "Transform Structure"))
  ;[1 0.2685 0.3296] Server-side RPC Handling
  (set `self.pawnTransform` transform))

(event `self.ReceiveTick`
  (params (DeltaSeconds :type "Float (single-precision)"))
  (bind _returnvalue (`self.GetLocalRole`))
  (bind _playerstate (`self.PlayerState`))
  (bind _playernamerender (`self.playerNameRender`))
  (`|ExecutionSequence`
    (:`then_0`
      ;[1 0.9635 0.1915] Replicate Pawn Transform by Calling RPC
      (if (or (`|EnumEquality` _returnvalue "ROLE_AutonomousProxy") (`|EnumEquality` _returnvalue "ROLE_Authority"))
        (`self.RPC Server Pawn Transform Replicate` (`KismetMathLibrary.MakeTransform` (.location (`self.GetTransform`)) (`SceneComponent.K2_GetComponentRotation` (`self.spectatorCamera`))))))
    (:`then_1`
      ;[1 1 1] Turn Player Name to Face Camera
      (`SceneComponent.K2_SetWorldRotation` _playernamerender (.rotation (`self.GetTransform` (`GameplayStatics.GetPlayerController` 0))) false false)
      (`SceneComponent.K2_AddLocalRotation` _playernamerender (struct :`Yaw` 180.0) false false))
    (:`then_2`
      ;[1 1 1] This is a one-time thing, but it can't be in BeginPlay nor OnPosessed, because for the former, player state is still null, for the latter - it won't be called for non-owning clients. So resort to ugly hack, well why am i surprised
      (if (`self.isNameRenderTextSet`)
        _
        (elif (`KismetSystemLibrary.IsValid` _playerstate)
          (bind _asbp_player_state (cast `/Game/Blueprints/BP_PlayerState` _playerstate))
          (`/Game/Blueprints/BP_PlayerState.Set Player Name Render Text` _asbp_player_state)
          (set `self.isNameRenderTextSet` true))))
    (:`then_3`
      ;[1 1 1] update camera rotation locally
      (`SceneComponent.K2_SetWorldRotation` (`self.spectatorCamera`) (.rotation (`self.pawnTransform`)) false false))))

(fn `OnRep_pawnTransform`
  (`self.K2_SetActorTransform` (`self.pawnTransform`)))

(fn `OnRep_playerName`)

(fn `UserConstructionScript`)