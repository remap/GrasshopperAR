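; Networked AR player pawn that shows each player as a cone avatar with axes and a name label, hidden in standalone and for the autonomous proxy.
; On Tick the owning client sends changed camera and pawn transforms through server RPCs, and OnRep functions apply them on non-owners.
; Tick also turns the name label toward the local camera and sets its text once PlayerState is valid.
; Touches line-trace into the world and broadcast the hit actor.
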(event `InputTouch`
  (params (Location :type "Vector Structure") (FingerIndex :type "ETouchIndex Enum"))
  (bind (_locationx _locationy) (`PlayerController.GetInputTouchState` (`GameplayStatics.GetPlayerController` 0) "Touch1"))
  ;[1 0.04705 0.1718] WORLD HIT TEST. Results delivered via ARHit Result Delegate
  (:`Pressed`
    (bind (_outhits _returnvalue) (`self.WorldHitTest` (`KismetMathLibrary.MakeVector2D` _locationx _locationy)))
    (if _returnvalue
      (`self.ARHitResult` (`.HitActor` (`GameplayStatics.BreakHitResult` (`|GetArrayItem` _outhits)))))))

(event `self.ReceiveBeginPlay`
  (bind _returnvalue (`self.GetLocalRole`))
  (bind _returnvalue_2 (`KismetTextLibrary.Conv_ByteToText` _returnvalue))
  (`DDBlueprintLibrary.LogDebug` (`KismetTextLibrary.Conv_TextToString` (`|FormatText` "AR Pawn BeginPlay. Net role {role} remote {remoteRole}" (`KismetMathLibrary.Conv_ByteToInt` (`self.GetLocalRole`)) (`KismetMathLibrary.Conv_ByteToInt` (`self.GetRemoteRole`)))))
  ;[1 1 1] toggle ar pawn rendering (red cone) depening on client/server role
  (bind _returnvalue_3 (`DDBlueprintLibrary.getGameNetMode`))
  (if (or (`KismetStringLibrary.EqualEqual_StrStr` _returnvalue_3 "NM_Standalone") (`|EnumEquality` _returnvalue "ROLE_AutonomousProxy"))
    (`DDBlueprintLibrary.LogDebug` (`KismetTextLibrary.Conv_TextToString` (`|FormatText` "Disable pawn rendering (mode {m} role {r})" _returnvalue_3 _returnvalue_2)))
    (`SceneComponent.SetVisibility` (`self.Cone`) false true)
    (`SceneComponent.SetVisibility` (`self.playerNameRender`) false true)
    (`SceneComponent.SetVisibility` (`self.PawnAxes`) false true)
    (else
      (`DDBlueprintLibrary.LogError` (`KismetTextLibrary.Conv_TextToString` (`|FormatText` "Enable pawn rendering.(mode {m} role {r})" _returnvalue_3 _returnvalue_2))))))

(event `RPC Server Camera Transform Replicate`
  (params (transform :type "Transform Structure"))
  ;[1 1 1] Server-side RPC Handling
  (set `self.cameraTransform` transform))

(event `self.ReceiveTick`
  (params (DeltaSeconds :type "Float (single-precision)"))
  (bind _returnvalue (`self.GetTransform`))
  (bind _playerstate (`self.PlayerState`))
  (bind _playernamerender (`self.playerNameRender`))
  (bind _returnvalue_2 (`SceneComponent.GetRelativeTransform` (`self.Camera`)))
  (`|ExecutionSequence`
    (:`then_0`
      ;[1 0.9076 0.1808] Replicate Relative Camera Transform
      (if (`|EnumEquality` (`self.GetLocalRole`) "ROLE_AutonomousProxy")
        (`|ExecutionSequence`
          (:`then_0`
            (if (not (`KismetMathLibrary.NearlyEqual_TransformTransform` (`self.cameraTransform`) _returnvalue_2 0.01 0.01 0.01))
              (bind _output_get (set `self.cameraTransform` _returnvalue_2))
              (`self.RPC Server Camera Transform Replicate` _output_get)))
          (:`then_1`
            (if (not (== (`self.pawnTransform`) _returnvalue))
              (bind _output_get_2 (set `self.pawnTransform` _returnvalue))
              (`self.RPC Server Pawn Transform Replicate` _output_get_2))))))
    (:`then_1`
      ;[1 1 1] Turn Player Name to Face Camera
      (`SceneComponent.K2_SetWorldRotation` _playernamerender (.rotation (`self.GetTransform` (`GameplayStatics.GetPlayerController` 0))) false false)
      (`SceneComponent.K2_AddLocalRotation` _playernamerender (struct :`Yaw` 180.0) false false))
    (:`then_2`
      (if (`self.isNameRenderTextSet`)
        _
        (elif (`KismetSystemLibrary.IsValid` _playerstate)
          (bind _asbp_player_state (cast `/Game/Blueprints/BP_PlayerState` _playerstate))
          (`/Game/Blueprints/BP_PlayerState.Set Player Name Render Text` _asbp_player_state)
          (set `self.isNameRenderTextSet` true))))))

(event `RPC Server Pawn Transform Replicate`
  (params (transform :type "Transform Structure"))
  ;[1 1 1] Server-side RPC Handling
  (set `self.pawnTransform` transform))

(fn `OnRep_cameraTransform`
  ;[1 1 1] This won't run on owner, because Camera Transform Replicate set to SkipOwner
  (if (not (`|EnumEquality` (`self.GetLocalRole`) "ROLE_AutonomousProxy"))
    (`SceneComponent.K2_SetRelativeTransform` (`self.Camera`) (`self.cameraTransform`) false false)))

(fn `OnRep_isAvatarHidden`)

(fn `OnRep_pawnTransform`
  (if (not (`|EnumEquality` (`self.GetLocalRole`) "ROLE_AutonomousProxy"))
    (`self.K2_SetActorTransform` (`self.pawnTransform`))))

(fn `UserConstructionScript`)

(fn `WorldHitTest`
  (params (ScreenPosition :type "Vector2D Structure"))
  (returns (OutHits :type "Array of HitResult Structure") (ReturnValue :type Boolean))
  (bind (_worldposition _worlddirection) (`GameplayStatics.DeprojectScreenToWorld` (`GameplayStatics.GetPlayerController` 0) ScreenPosition))
  (bind (_outhits _returnvalue) (`KismetSystemLibrary.LineTraceMultiForObjects` _worldposition (+ _worldposition (* _worlddirection 1000.0)) (`|MakeArray` "ObjectTypeQuery1" "ObjectTypeQuery2" "ObjectTypeQuery3" "ObjectTypeQuery4" "ObjectTypeQuery5" "ObjectTypeQuery6" :!type "EObjectTypeQuery Enum")))
  (return _outhits _returnvalue))