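; Blueprint helper library for finding player starts by tag and moving a player to one.
; The lookup returns the first tagged actor cast to PlayerStart, with a Print Starts helper logging level info when several match.
; The move teleports the player's controlled pawn to a valid start's location without changing rotation.
; Both functions log problems such as missing tags, wrong classes or failed moves.
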(fn `Get Player Start With Tag`
  (params (tag :type Name))
  (returns (playerStart :type "PlayerStart Object Reference"))
  (bind _outactors (`GameplayStatics.GetAllActorsWithTag` null tag))
  (bind _returnvalue (`KismetArrayLibrary.Array_Length` _outactors))
  (if (> _returnvalue 0)
    (if (> _returnvalue 1)
      (`DDBlueprintLibrary.LogDebug` "FOUND MORE STARTS")
      (for (_array_element _array_index) _outactors
        (bind _returnvalue_2 (`GameplayStatics.GetCurrentLevelName` _array_element false))
        (`DDBlueprintLibrary.LogInfo` (`KismetTextLibrary.Conv_TextToString` (`|FormatText` "Start {index} level name {level} " _array_index (`KismetTextLibrary.Conv_StringToText` _returnvalue_2))))
        (bind _asplayer_start (cast `PlayerStart` (`|GetArrayItem` _outactors) :!label _label)
          (:`then`
            _)
          (:`CastFailed`
            (`DDBlueprintLibrary.LogError` "Tagged actor is not a player start class")))
        (return _asplayer_start))
      (else
        (goto _label)))
    (else
      (`DDBlueprintLibrary.LogWarning` (`KismetTextLibrary.Conv_TextToString` (`|FormatText` "Couldn't find player start with tag {tag}" (`KismetTextLibrary.Conv_NameToText` tag))))
      (return null))))

(fn `Move Player To Start`
  (params (player :type "PlayerController Object Reference") (playerStart :type "Actor Object Reference"))
  (returns (moved :type Boolean))
  (bind _returnvalue (`Actor.K2_GetActorLocation` playerStart))
  (if (`KismetSystemLibrary.IsValid` playerStart)
    (bind (_sweephitresult _returnvalue_2) (`Actor.K2_SetActorLocation` (`Controller.K2_GetPawn` player) _returnvalue false true))
    (if _returnvalue_2
      (`DDBlueprintLibrary.LogDebug` (`KismetTextLibrary.Conv_TextToString` (`|FormatText` "Player moved successfully to {location}" (`KismetTextLibrary.Conv_VectorToText` _returnvalue))))
      (return true)
      (else
        (`DDBlueprintLibrary.LogError` "Player move FAILED")
        (return false)))))