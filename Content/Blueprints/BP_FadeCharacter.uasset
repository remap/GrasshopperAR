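; BP_FadeCharacter is an actor that plays a video with a separate alpha video on a plane, likely a recorded character cutout.
; On BeginPlay it creates an M_MaskedVideo dynamic material, binds both media textures to their players, then opens and plays both sources.
; FlipTextureHorizonal swaps the u1/u2 material parameters to mirror the image, optionally at startup.
; The Dissolve parameter setter is unconnected, so no fade runs here.
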(event `self.ReceiveBeginPlay`
  (bind _mediaplayer_aplha (`self.MediaPlayer_Aplha`))
  (bind _mediaplayer (`self.MediaPlayer`))
  (bind _mediaalpha_tex (`self.MediaAlpha_Tex`))
  (bind _media_tex (`self.Media_Tex`))
  (`|ExecutionSequence`
    (:`then_0`
      (bind _returnvalue (`PrimitiveComponent.CreateDynamicMaterialInstance` (`self.Plane`) 0 "/Game/AJAX/VIDEO/Vid_Material/M_MaskedVideo.M_MaskedVideo" "None"))
      (bind _output_get (set `self.MaterialInstance` _returnvalue))
      (`/Engine/EditorBlueprintResources/StandardMacros.IsValid` _media_tex
        (:`Is Valid`
          (`/Engine/EditorBlueprintResources/StandardMacros.IsValid` _mediaalpha_tex
            (:`Is Valid`
              (`MaterialInstanceDynamic.SetTextureParameterValue` _output_get "Video" _media_tex)
              (`MaterialInstanceDynamic.SetTextureParameterValue` _output_get "Video_Alpha" _mediaalpha_tex)
              (`MediaTexture.SetMediaPlayer` _media_tex (`self.MediaPlayer`))
              (`MediaTexture.SetMediaPlayer` _mediaalpha_tex (`self.MediaPlayer_Aplha`))
              (if (`self.FlipHorizontal On Construct`)
                (`self.Flip Texture Horizonal`)))))))
    (:`then_1`
      (`MediaPlayer.OpenSource` _mediaplayer (`self.FileMediaSource`))
      (`MediaPlayer.Play` _mediaplayer))
    (:`then_2`
      (`MediaPlayer.OpenSource` _mediaplayer_aplha (`self.MediaSource_Alpha`))
      (`MediaPlayer.Play` _mediaplayer_aplha))))

(fn `Flip Texture Horizonal`
  (bind _materialinstance (`self.MaterialInstance`))
  (bind _isa (`/Engine/EditorBlueprintResources/StandardMacros.FlipFlop`)
    (:`A`
      _)
    (:`B`
      _))
  (bind _returnvalue (`KismetMathLibrary.SelectFloat` 1.0 0.0 _isa))
  (`MaterialInstanceDynamic.SetScalarParameterValue` _materialinstance "u1" _returnvalue)
  (`MaterialInstanceDynamic.SetScalarParameterValue` _materialinstance "u2" (- 1.0 _returnvalue)))

(fn `Initialize Recorded Plane`)

(fn `UserConstructionScript`)