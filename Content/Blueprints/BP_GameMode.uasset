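; Game mode for a cross-platform AR/VR project that picks player starts by controller type.
; BeginPlay branches on platform name, logging AR mode for iOS and Android, VR mode for Mac and Windows, and a warning otherwise.
; The platform branches only log, and OnPlatformSetupComplete is an empty stub.
; ChoosePlayerStart casts to BP_VRController or BP_ARController and returns that controller's PlayerStart, logging missing starts or unknown controllers.
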(event `self.ReceiveBeginPlay`
  (bind _returnvalue (`GameplayStatics.GetPlatformName`))
  (bind _returnvalue_2 (`KismetTextLibrary.Conv_StringToText` _returnvalue))
  (bind _returnvalue_3 (`KismetTextLibrary.Conv_TextToString` (`|FormatText` "Running on {Platform}" _returnvalue_2)))
  (`|ExecutionSequence`
    (:`then_0`
      ;[0.7985 0.3799 1] Platform Specific Setup
      (`DDBlueprintLibrary.LogDebug` "GAME MODE BEGIN PLAY")
      (switch `string` _returnvalue
        (:`Default`
          (`DDBlueprintLibrary.LogWarning` (`KismetTextLibrary.Conv_TextToString` (`|FormatText` "Unsupported platform: {Platform}" _returnvalue_2))))
        (:`IOS`
          (`DDBlueprintLibrary.LogDebug` _returnvalue_3 :!label _label)
          (`|ExecutionSequence`
            (:`then_0`
              (`DDBlueprintLibrary.LogDebug` "Starting AR mode"))))
        (:`Android`
          (goto _label))
        (:`Mac`
          (`DDBlueprintLibrary.LogDebug` _returnvalue_3 :!label _label_2)
          (`|ExecutionSequence`
            (:`then_0`
              (`DDBlueprintLibrary.LogDebug` "Starting VR mode"))))
        (:`Windows`
          (goto _label_2))))))

(event `On Platform Setup Complete`
  ;[0.2074 1 0.2958] Platform Agnostic Setup
)

(fn `ChoosePlayerStart`
  (params (Player :type "Controller Object Reference"))
  (returns (ReturnValue :type "Actor Object Reference"))
  (`DDBlueprintLibrary.LogDebug` (`KismetTextLibrary.Conv_TextToString` (`|FormatText` "Choose player start for controller {controller}" (`KismetTextLibrary.Conv_StringToText` (`KismetSystemLibrary.GetClassDisplayName` (`GameplayStatics.GetObjectClass` Player))))))
  ;[1 1 1] Return VR Player Start
  (bind _asbp_vrcontroller (cast `/Game/Blueprints/BP_VRController` Player)
    (:`then`
      (bind _playerstart (`GHBasePlayerController.playerStart` _asbp_vrcontroller))
      (if (`KismetSystemLibrary.IsValid` _playerstart)
        (`DDBlueprintLibrary.LogDebug` (`KismetTextLibrary.Conv_TextToString` (`|FormatText` "Player start at {transform}" (`KismetTextLibrary.Conv_TransformToText` (`self.GetTransform` _playerstart)))))
        (else
          (`DDBlueprintLibrary.LogError` "VR Player Start is NULL ")))
      (return _playerstart))
    (:`CastFailed`
      ;[1 1 1] Return AR Player Start
      (bind _asbp_arcontroller (cast `/Game/Blueprints/BP_ARController` Player)
        (:`then`
          (bind _playerstart_2 (`GHBasePlayerController.playerStart` _asbp_arcontroller))
          (if (not (`KismetSystemLibrary.IsValid` _playerstart_2))
            (`DDBlueprintLibrary.LogError` "AR Player Start is NULL")))
        (:`CastFailed`
          (`DDBlueprintLibrary.LogWarning` "Failed to determine player controller")))
      (return _playerstart_2))))

(fn `UserConstructionScript`)