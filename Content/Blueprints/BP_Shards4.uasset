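; BP_Shards4 is a Blueprint that starts front and reverse video playback for what its name suggests is a shards piece.
; BeginPlay opens each media source on its own media player, then sets looping and plays it only if LevelLoaded is true.
; The check that would set LevelLoaded from the game instance for level AR_4_Scenic_Dev is disconnected, so playback depends on that variable's existing value.
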(event `self.ReceiveBeginPlay`
  (bind _islooping (`self.isLooping`))
  (bind _mediaplayerreverse (`self.mediaPlayerReverse`))
  (bind _mediaplayerfront (`self.mediaPlayerFront`))
  (`|ExecutionSequence`
    (:`then_0`
      (`MediaPlayer.OpenSource` _mediaplayerfront (`self.mediaSourceFront`))
      (if (`self.levelLoaded`)
        (`MediaPlayer.SetLooping` _mediaplayerfront _islooping)
        (`MediaPlayer.Play` (`self.mediaPlayerFront`))))
    (:`then_1`
      (`MediaPlayer.OpenSource` _mediaplayerreverse (`self.mediaSourceReverse`))
      (if (`self.levelLoaded`)
        (`MediaPlayer.SetLooping` _mediaplayerreverse _islooping)
        (`MediaPlayer.Play` _mediaplayerreverse)))))

(event `self.ReceiveTick`
  (params (DeltaSeconds :type "Float (single-precision)")))

(fn `UserConstructionScript`)