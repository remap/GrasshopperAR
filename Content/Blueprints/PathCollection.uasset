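; PathCollection is an actor that generates light paths radiating out from itself and reveals them when another actor overlaps it.
; On BeginPlay, if Random is set, it picks random flat endpoints and builds a jittered spline to each from the local origin.
; Each spline is handed to a spawned, owned LightPaths actor.
; Reveal calls FadePath on every stored path, which overlap triggers at full ratio.
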(event `self.ReceiveBeginPlay`
  (bind (_returnvalue_x _returnvalue_y) (`KismetMathLibrary.BreakVector` (`KismetMathLibrary.RandomUnitVector`)))
  (bind _endpoints (`self.endpoints`))
  (if (`self.Random`)
    (for _ (range (+ (`self.numPaths`) 1))
      (`KismetArrayLibrary.Array_Add` _endpoints (`KismetMathLibrary.MakeVector` (* (`KismetMathLibrary.RandomIntegerInRange` 400 500) _returnvalue_x) (* (`KismetMathLibrary.RandomIntegerInRange` 400 600) _returnvalue_y))))
    (for (_ _array_index) _endpoints
      (bind _returnvalue (`AddComponent|NODE_AddSplineComponent-2`))
      (bind _mesh (`self.makePath` _array_index _returnvalue))
      (`/Engine/EditorBlueprintResources/StandardMacros.IsValid` _mesh
        (:`Is Valid`
          (`KismetArrayLibrary.Array_Add` (`self.paths`) _mesh))))))

(event `self.ReceiveActorBeginOverlap`
  (params (OtherActor :type "Actor Object Reference"))
  (`self.reveal` 1.0))

(fn `addRandomPoints`
  (params (endpoint :type "Vector Structure") (numPoints :type Integer) (randomness :type Integer))
  (returns (returnPoints :type "Array of Vector Structure"))
  (locals (points :type "Array of Vector Structure"))
  (bind (_returnvalue_x _returnvalue_y) (`KismetMathLibrary.BreakVector` (* (`KismetMathLibrary.RandomUnitVector`) (`KismetMathLibrary.RandomInteger` (* randomness 2)))))
  (for _index (range (+ numPoints 1))
    (`KismetArrayLibrary.Array_AddUnique` (`local.points`) (+ (`KismetMathLibrary.VLerp` (0.0 0.0 0.0) endpoint (`KismetMathLibrary.RandomFloatInRange` (/ (`KismetMathLibrary.Conv_IntToDouble` _index) (`KismetMathLibrary.Conv_IntToDouble` numPoints)) (/ (`KismetMathLibrary.Conv_IntToDouble` (+ _index 1)) (`KismetMathLibrary.Conv_IntToDouble` numPoints)))) (`KismetMathLibrary.MakeVector` _returnvalue_x _returnvalue_y))))
  (`KismetArrayLibrary.Array_AddUnique` (`local.points`) (`local.endpoint`))
  (return (`local.points`)))

(fn `makePath`
  (params (index :type Integer) (spline :type "SplineComponent Object Reference"))
  (returns (mesh :type "/Game/Blueprints/LightPaths Object Reference"))
  (bind _returnpoints (`self.addRandomPoints` (`|GetArrayItem` (`self.endpoints`) index) 4 30))
  (`SplineComponent.SetSplinePoints` spline _returnpoints "Local" true)
  (bind _returnvalue (`|SpawnActorFromClass` "/Game/Blueprints/LightPaths.LightPaths_C" (`self.GetTransform`) "AlwaysSpawn" "OverrideRootScale" null spline null))
  (`self.SetOwner` _returnvalue self)
  (return _returnvalue))

(fn `reveal`
  (params (ratio :type "Float (double-precision)") (rate :type "Float (double-precision)"))
  (for _array_element (`self.paths`)
    (`/Game/Blueprints/LightPaths.fadePath` _array_element ratio rate)))

(fn `UserConstructionScript`
  (locals (NewLocalVar_0 :type "Array of Vector Structure")))