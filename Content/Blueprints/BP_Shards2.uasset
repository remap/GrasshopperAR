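; BP_Shards2 is an actor Blueprint that starts media playlist playback on BeginPlay.
; It opens MediaPlaylist on its MediaPlayer, then calls Play only if the LevelLoaded flag is true.
; The game instance check that would set LevelLoaded from the AR_4_Scenic_Main level is unconnected and never runs, so playback relies on the flag's existing value.
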(event `self.ReceiveBeginPlay`
  (`|ExecutionSequence`
    (:`then_0`
      (`MediaPlayer.OpenPlaylist` (`self.mediaPlayer`) (`self.mediaPlaylist`))
      (if (`self.levelLoaded`)
        (`MediaPlayer.Play` (`self.mediaPlayer`))))))

(event `self.ReceiveTick`
  (params (DeltaSeconds :type "Float (single-precision)")))

(fn `UserConstructionScript`)