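; Actor component that auto-rotates its owner, normally a BP_PlaneBase whose built-in autorotate it disables, to face the player camera.
; Tick activates it within an optional radius and runs the selected mode, with optional axis-constrained look-at.
; Default tracks continuously, Type 1 pauses in a dead zone then flips 180° relative to the activation transform, and Type 2 flips past an angle from the original transform.
; DebugView draws axes and thresholds.
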(event `self.ReceiveBeginPlay`
  (bind _returnvalue (`self.GetOwner`))
  (bind _asbp_plane_base (cast `/VideoCore/Blueprints/BP_PlaneBase` _returnvalue)
    (:`then`
      (set `self.owner` _asbp_plane_base)
      ;[1 1 1] disable plane autorotate, since it'll be handled by this component
      (set `/VideoCore/Blueprints/BP_PlaneBase.isAutoRotate` false _asbp_plane_base)
      (set `/VideoCore/Blueprints/BP_PlaneBase.isInvertedAutorotate` false _asbp_plane_base))
    (:`CastFailed`
      (set `self.owner` _returnvalue)
      (`DDBlueprintLibrary.LogWarning` "Plane Autorotate Component not attached to a plane")))
  (set `self.planeOriginalT` (`self.Get Owner T`)))

(event `On Autorotate Activate`
  ;[1 0.6432 0.4077] on activate / deactivate
  (set `self.onActivateT` (`self.Get Owner T`))
  (`DDBlueprintLibrary.LogInfo` "A/R Active"))

(event `self.ReceiveTick`
  (params (DeltaSeconds :type "Float (single-precision)"))
  (bind _isactive (`self.Is Autorotation Active`))
  (`|ExecutionSequence`
    (:`then_0`
      (`self.Print Debug Info`))
    (:`then_1`
      (if (xor _isactive (`self.lastActiveState`))
        (if _isactive
          (`self.On Autorotate Activate`)
          (else
            (`self.On Autorotate Deactivate`))))
      (set `self.lastActiveState` _isactive))
    (:`then_2`
      (if _isactive
        (switch `/Game/Blueprints/PlaneComponents/E_PlaneAutorotate` (`self.autorotation`)
          (:`NewEnumerator1`
            (`self.Handle Autorotation Default`))
          (:`NewEnumerator2`
            (`self.Handle Autorotation Type1`))
          (:`NewEnumerator3`
            (`self.Handle Autorotation Type2`)))))))

(event `On Autorotate Deactivate`
  ;[1 0.6432 0.4077] on activate / deactivate
  (set `self.onDeactivateT` (`self.Get Owner T`))
  (set `self.isInDeadZone` false)
  (`DDBlueprintLibrary.LogInfo` "A/R Deactivated"))

(fn `Draw Debug Arrow`
  (params (v :type "Vector Structure") (len :type "Float (double-precision)" :default 100.0) (LineColor :type "LinearColor Structure") (Thickness :type "Float (double-precision)" :default 2.0) (Duration :type "Float (double-precision)"))
  (bind _loc (`self.Get Owner Loc`))
  (`KismetSystemLibrary.DrawDebugArrow` _loc (+ _loc (* v len)) 0.0 LineColor Duration Thickness))

(fn `Flip Owner`
  (if (== (.yaw (`self.flipOffset`)) 0.0)
    (set `self.flipOffset` (`KismetMathLibrary.MakeRotator` 0.0 0.0 180.0))
    (`DDBlueprintLibrary.LogDebug` "Flip to back")
    (else
      (set `self.flipOffset` (`KismetMathLibrary.MakeRotator` 0.0))
      (`DDBlueprintLibrary.LogDebug` "Flip to front"))))

(fn `Get Look At V`
  (returns (v :type "Vector Structure"))
  (return (`KismetMathLibrary.Normal` (- (`self.Get Player Camera Location`) (`self.Get Owner Loc`)))))

(fn `Get Owner Fw V`
  (returns (v :type "Vector Structure"))
  (return (`SceneComponent.GetForwardVector` (`Actor.RootComponent` (`self.owner`)))))

(fn `Get Owner Loc`
  (returns (loc :type "Vector Structure"))
  (return (`SceneComponent.K2_GetComponentLocation` (`Actor.RootComponent` (`self.owner`)))))

(fn `Get Owner Right V`
  (returns (v :type "Vector Structure"))
  (return (`SceneComponent.GetRightVector` (`Actor.RootComponent` (`self.owner`)))))

(fn `Get Owner T`
  (returns (t :type "Transform Structure"))
  (return (`SceneComponent.K2_GetComponentToWorld` (`Actor.RootComponent` (`self.owner`)))))

(fn `Get Owner Up V`
  (returns (v :type "Vector Structure"))
  (return (`SceneComponent.GetUpVector` (`Actor.RootComponent` (`self.owner`)))))

(fn `Get Player Camera Location`
  (returns (playerLocation :type "Vector Structure"))
  (return (`PlayerCameraManager.GetCameraLocation` (`PlayerController.PlayerCameraManager` (`GameplayStatics.GetPlayerController` 0)))))

(fn `Get Rotation Angle From T`
  (params (T :type "Transform Structure (by ref)"))
  (returns (ReturnValue :type "Float (double-precision)"))
  (return (`KismetMathLibrary.DegAcos` (`KismetMathLibrary.Vector_CosineAngle2D` (`self.projected` (`KismetMathLibrary.TransformDirection` T (`KismetMathLibrary.MakeVector` 1.0))) (`self.projected` (- (`self.Get Player Camera Location`) (`self.Get Owner Loc`)))))))

(fn `Get Type 1 DeadZone V`
  (params (invert :type Boolean))
  (returns (v :type "Vector Structure"))
  (return (`KismetMathLibrary.RotateAngleAxis` (`self.projected` (`KismetMathLibrary.TransformDirection` (`self.onActivateT`) (`KismetMathLibrary.MakeVector` 1.0))) (* (select `bool` invert :`false` 1 :`true` -1) (+ (`self.type1Alpha`) (`self.type1DeadZone`))) (0.0 0.0 1.0))))

(fn `Get Type1 Alpha V`
  (params (invert :type Boolean))
  (returns (v :type "Vector Structure"))
  (return (`KismetMathLibrary.RotateAngleAxis` (`self.projected` (`KismetMathLibrary.TransformDirection` (`self.onActivateT`) (`KismetMathLibrary.MakeVector` 1.0))) (* (select `bool` invert :`false` 1 :`true` -1) (`self.type1Alpha`)) (0.0 0.0 1.0))))

(fn `Handle Autorotation Default`
  (bind _rootcomponent (`Actor.RootComponent` (`self.owner`)))
  (`self.Set Owner Look At` (`self.Get Player Camera Location`))
  (`SceneComponent.K2_AddLocalRotation` _rootcomponent (`self.localRotationOffset`) false false)
  (`SceneComponent.K2_AddLocalRotation` _rootcomponent (`self.flipOffset`) false false))

(fn `Handle Autorotation Type1`
  (locals (currentAngle :type "Float (double-precision)") (greaterThanAlpha :type "Float (double-precision)"))
  (bind _output_get (set `local.currentAngle` (`self.Get Rotation Angle From T` (`self.onActivateT`))))
  (if (>= _output_get (`self.type1Alpha`))
    (if (`self.isInDeadZone`)
      (if (>= (`local.currentAngle`) (+ (`self.type1Alpha`) (`self.type1DeadZone`)))
        (set `self.isInDeadZone` false)
        (`self.Flip Owner`)
        (`self.Set Owner Look At` (`self.Get Player Camera Location`))
        (set `self.onActivateT` (`self.Get Owner T`)))
      (else
        (set `self.isInDeadZone` true)))
    (else
      (set `self.isInDeadZone` false)
      (`self.Handle Autorotation Default`))))

(fn `Handle Autorotation Type2`
  (locals (currentAngle :type "Float (double-precision)") (flipAngleThreshold :type "Float (double-precision)" :default 90.0))
  (bind _returnvalue (`self.Get Rotation Angle From T` (`self.planeOriginalT`)))
  (if (== (.yaw (`self.flipOffset`)) 180.0)
    (set `local.currentAngle` (- 180.0 _returnvalue))
    (else
      (bind _output_get (set `local.currentAngle` _returnvalue))))
  (if (> _output_get (`local.flipAngleThreshold`))
    (`self.Flip Owner`)
    (else
      (`self.Handle Autorotation Default`))))

(fn `Is Autorotation Active`
  (returns (isActive :type Boolean))
  (bind _activateradius (`self.activateRadius`))
  (if (> _activateradius 0.0)
    (return (<= (`KismetMathLibrary.Vector_Distance` (`self.Get Player Camera Location`) (`Actor.K2_GetActorLocation` (`self.owner`))) _activateradius))
    (else
      (return true))))

(fn `Print Debug Info`
  (locals (localCenter :type "Vector Structure") (planeFw :type "Vector Structure") (planeUp :type "Vector Structure") (planeRight :type "Vector Structure"))
  (bind _planeoriginalt (`self.planeOriginalT`))
  (bind _localcenter (`local.localCenter`))
  (bind _localcenter_2 (`local.localCenter`))
  (bind _rootcomponent (`Actor.RootComponent` (`self.owner`)))
  (bind _returnvalue (* (`self.projected` (`KismetMathLibrary.TransformDirection` _planeoriginalt (`KismetMathLibrary.MakeVector` 0.0 1.0))) 120.0))
  (if (`self.debugView`)
    (set `local.localCenter` (`SceneComponent.K2_GetComponentLocation` _rootcomponent))
    (set `local.planeFw` (`self.projected` (`SceneComponent.GetForwardVector` _rootcomponent)))
    (set `local.planeUp` (`SceneComponent.GetUpVector` _rootcomponent))
    (set `local.planeRight` (`self.projected` (`SceneComponent.GetRightVector` _rootcomponent)))
    (`|ExecutionSequence`
      (:`then_0`
        (`KismetSystemLibrary.DrawDebugCircle` _localcenter_2 70.0 72 (struct :`G` 0.552083 :`B` 0.052231 :`A` 1.0) 0.0 1.0 (`local.planeRight`) (`local.planeFw`) true)
        (`KismetSystemLibrary.DrawDebugCoordinateSystem` _localcenter_2 (struct) 100.0 0.0 1.0)
        (`KismetSystemLibrary.DrawDebugLine` _localcenter (+ _localcenter _returnvalue) (struct :`R` 1.0 :`G` 0.207749 :`A` 1.0) 0.0 2.0)
        (`KismetSystemLibrary.DrawDebugLine` _localcenter (- _localcenter _returnvalue) (struct :`R` 1.0 :`G` 0.207749 :`A` 1.0) 0.0 2.0)
        (`self.Draw Debug Arrow` (`KismetMathLibrary.TransformDirection` _planeoriginalt (`KismetMathLibrary.MakeVector` 1.0)) 120.0 (struct :`R` 1.0 :`G` 0.139721 :`A` 1.0)))
      (:`then_1`
        (`self.Draw Debug Arrow` (`local.planeFw`) 100.0 (select `bool` (`self.Is Autorotation Active`) :`false` (struct :`R` 0.099115 :`G` 0.126638 :`B` 0.796875 :`A` 1.0) :`true` (struct :`R` 0.103198 :`G` 1.0 :`B` 0.960197 :`A` 1.0) :!type "LinearColor Structure"))
        (`self.Draw Debug Arrow` (`self.projected` (`self.Get Look At V`)) 150.0 (struct :`R` 0.984375 :`B` 0.027913 :`A` 1.0) 1.0 (select `bool` (`self.isInDeadZone`) :`true` 1.0 :!type "Float (single-precision)")))
      (:`then_2`
        (switch `/Game/Blueprints/PlaneComponents/E_PlaneAutorotate` (`self.autorotation`)
          (:`NewEnumerator2`
            (if (`self.Is Autorotation Active`)
              (`self.Draw Debug Arrow` (`self.Get Type1 Alpha V` false) 100.0 (struct :`R` 0.9375 :`G` 0.059191 :`B` 0.764104 :`A` 1.0))
              (`self.Draw Debug Arrow` (`self.Get Type1 Alpha V` true) 100.0 (struct :`R` 0.9375 :`G` 0.059191 :`B` 0.764104 :`A` 1.0))
              (`self.Draw Debug Arrow` (`self.Get Type 1 DeadZone V` false) 100.0 (struct :`R` 0.9375 :`G` 0.855638 :`B` 0.027042 :`A` 1.0))
              (`self.Draw Debug Arrow` (`self.Get Type 1 DeadZone V` true) 100.0 (struct :`R` 0.9375 :`G` 0.855638 :`B` 0.027042 :`A` 1.0)))))))))

(fn `Set Owner Look At`
  (params (InputPin :type "Vector Structure"))
  (bind _owner (`self.owner`))
  (`self.Is Axis Constraint Autorotation ?`
    (:`ayeah`
      (`SceneComponent.K2_AddLocalRotation` (`Actor.RootComponent` (`self.owner`)) (`KismetMathLibrary.FindLookAtRotation` (`KismetMathLibrary.MakeVector` 0.0) (`KismetMathLibrary.ProjectPointOnToPlane` (.location (`KismetMathLibrary.MakeRelativeTransform` (`KismetMathLibrary.Conv_VectorToTransform` InputPin) (`self.Get Owner T`))) (0.0 0.0 0.0) (`self.autorotateAxis`))) false false))
    (:`nah`
      (`SceneComponent.K2_SetWorldRotation` (`Actor.RootComponent` _owner) (`KismetMathLibrary.FindLookAtRotation` (`Actor.K2_GetActorLocation` _owner) InputPin) false false)))
  (return))