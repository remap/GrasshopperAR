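; SwitchVideoComponent swaps the video playing on its owning BP_RecordedPlane, taking the plane's media player and texture on BeginPlay.
; SwitchVideo opens the indexed source in a newly constructed MediaPlayer with seek and loop options, while the current player stays in place.
; Once that opens, after an optional delay, it pauses the old player, sets playback speed and repoints the texture, plane reference and media sound to the new one.
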(event `self.ReceiveBeginPlay`
  (`self.InitFromOwningRecordedPlane`))

(event `Switch Video`
  (params (Params :type "/Game/Cues/Parameters/SwitchVideoParams Structure"))
  (bind (_mediasource _mediaplayeroptions) (`self.Parse Params`))
  (set `self.Params` Params)
  (bind _returnvalue (`|GenericCreateObject` "/Script/MediaAssets.MediaPlayer" self))
  (bind _output_get (set `self.ReplacementMediaPlayer` _returnvalue))
  (add `MediaPlayer.OnMediaOpened` _output_get (delegate `OnMediaOpened`))
  (`/Engine/EditorBlueprintResources/StandardMacros.IsValid` _mediasource
    (:`Is Valid`
      (`MediaPlayer.OpenSourceWithOptions` (`self.ReplacementMediaPlayer`) _mediasource _mediaplayeroptions))
    (:`Is Not Valid`
      (`KismetSystemLibrary.PrintString` "SwitchVideoComponent: File not found"))))

(event `OnMediaOpened`
  (params (OpenedUrl :type String))
  (bind (_params_tag _params_delaytime _params_videoindex _params_islooping _params_seekpos _params_playbackspeed) (break `/Game/Cues/Parameters/SwitchVideoParams` (`self.Params`)))
  (bind (_params_tag_2 _params_delaytime_2) (break `/Game/Cues/Parameters/SwitchVideoParams` (`self.Params`)))
  (`KismetSystemLibrary.Delay` _params_delaytime_2)
  (`MediaPlayer.Pause` (`self.ActorMediaPlayer`))
  (bind _output_get (set `self.ActorMediaPlayer` (`self.ReplacementMediaPlayer`)))
  (`MediaPlayer.SetRate` _output_get _params_playbackspeed)
  (`MediaTexture.SetMediaPlayer` (`self.ActorMediaTexture`) (`self.ReplacementMediaPlayer`))
  (bind _asbp_recorded_plane (cast `/VideoCore/Blueprints/BP_RecordedPlane` (`self.GetOwner`)))
  (bind _output_get_2 (set `/VideoCore/Blueprints/BP_RecordedPlane.mediaPlayer` (`self.ActorMediaPlayer`) _asbp_recorded_plane))
  (`MediaSoundComponent.SetMediaPlayer` (`/VideoCore/Blueprints/BP_RecordedPlane.MediaSound` _asbp_recorded_plane) _output_get_2))

(fn `InitFromOwningRecordedPlane`
  (bind _asbp_recorded_plane (cast `/VideoCore/Blueprints/BP_RecordedPlane` (`self.GetOwner`)))
  (`|ExecutionSequence`
    (:`then_0`
      (`self.ActorMediaPlayer`
        (:`then`)
        (:`else`
          (set `self.ActorMediaPlayer` (`/VideoCore/Blueprints/BP_RecordedPlane.Get Media Player` _asbp_recorded_plane)))))
    (:`then_1`
      (`self.ActorMediaTexture`
        (:`then`)
        (:`else`
          (set `self.ActorMediaTexture` (`/VideoCore/Blueprints/BP_RecordedPlane.Get Media Texture` _asbp_recorded_plane)))))))

(fn `Parse Params`
  (returns (MediaSource :type "FileMediaSource Object Reference") (MediaPlayerOptions :type "MediaPlayerOptions Structure"))
  (bind (_tag _delaytime _videoindex _islooping _seekpos) (break `/Game/Cues/Parameters/SwitchVideoParams` (`self.Params`)))
  (return (`|GetArrayItem` (`self.MediaSources`) _videoindex) (make `MediaPlayerOptions` (struct :`Caption` -1 :`Metadata` -1 :`Script` -1 :`Subtitle` -1 :`Text` -1) (`KismetMathLibrary.MakeTimespan` 0 0 0 (`KismetMathLibrary.FTrunc` _seekpos)) "Enabled" (select `bool` _islooping :`false` "Disabled" :`true` "Enabled" :!type "EMediaPlayerOptionBooleanOverride Enum"))))