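; LightPaths is a spline-based path actor whose meshes fade through a dissolve material.
; The construction script adds a spline mesh per spline point, using an assigned Spline when valid.
; BeginPlay gives each mesh a dynamic MI_Dissolve instance with start and end values normalised along the spline length.
; FadePath sets a target, and Tick moves the shared cutoff toward it at FadeRate, updating every material.
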(event `self.ReceiveBeginPlay`
  (bind _spline1 (`self.Spline1`))
  (bind _returnvalue (`SplineComponent.GetSplineLength` _spline1))
  (for (_array_element _array_index) (`self.meshes`)
    (bind _returnvalue_2 (`KismetMaterialLibrary.CreateDynamicMaterialInstance` "/Game/Materials/AR_Assets/MI_Dissolve.MI_Dissolve"))
    (`PrimitiveComponent.SetMaterial` _array_element 0 _returnvalue_2)
    (`MaterialInstanceDynamic.SetScalarParameterValue` _returnvalue_2 "start" (/ (`SplineComponent.GetDistanceAlongSplineAtSplinePoint` _spline1 (- _array_index 1)) _returnvalue))
    (`MaterialInstanceDynamic.SetScalarParameterValue` _returnvalue_2 "end" (/ (`SplineComponent.GetDistanceAlongSplineAtSplinePoint` _spline1 _array_index) _returnvalue))
    (`MaterialInstanceDynamic.SetScalarParameterValue` _returnvalue_2 "cutoff" (`self.current`))
    (`BlueprintMapLibrary.Map_Add` (`self.mats`) _array_index _returnvalue_2)
    (`BlueprintMapLibrary.Map_Add` (`self.currentMap`) _array_index (`self.current`))))

(event `self.ReceiveTick`
  (params (DeltaSeconds :type "Float (single-precision)"))
  (bind _mats (`self.mats`))
  (if (not (== (`self.current`) (`self.fading`)))
    (if (< (`self.current`) (`self.fading`))
      (set `self.current` (`KismetMathLibrary.FClamp` (+ (`self.current`) (* DeltaSeconds (`self.fade rate`))) 0.0 1.5))
      (else
        (set `self.current` (`KismetMathLibrary.FClamp` (- (`self.current`) (* DeltaSeconds (`self.fade rate`))) 0.0 1.5))))
    (bind _keys (`BlueprintMapLibrary.Map_Keys` _mats))
    (for _array_element _keys
      (bind (_value _returnvalue) (`BlueprintMapLibrary.Map_Find` _mats _array_element))
      (if _returnvalue
        (`MaterialInstanceDynamic.SetScalarParameterValue` _value "cutoff" (`self.current`))))))

(event `self.ReceiveActorBeginOverlap`
  (params (OtherActor :type "Actor Object Reference")))

(fn `fadePath`
  (params (target :type "Float (double-precision)"))
  (set `self.fading` target)
  (set `self.counter` 0))

(fn `UserConstructionScript`
  (bind _spline1 (`self.Spline1`))
  (bind _spline (`self.Spline`))
  (`/Engine/EditorBlueprintResources/StandardMacros.IsValid` _spline
    (:`Is Valid`
      (set `self.Spline1` _spline))
    (:`Is Not Valid`
      _))
  (for _index (range (+ (`SplineComponent.GetNumberOfSplinePoints` (`self.Spline1`)) 1))
    (bind _returnvalue (`AddComponent|NODE_AddSplineMeshComponent-0` :`bManualAttachment` true))
    (`SceneComponent.K2_AttachToComponent` _returnvalue (`self.Spline1`) "None" "KeepRelative" "KeepRelative" "KeepRelative" true)
    (bind (_location _tangent) (`SplineComponent.GetLocationAndTangentAtSplinePoint` _spline1 _index "Local"))
    (bind (_location_2 _tangent_2) (`SplineComponent.GetLocationAndTangentAtSplinePoint` _spline1 (+ _index 1) "Local"))
    (`SplineMeshComponent.SetStartAndEnd` _returnvalue _location _tangent _location_2 _tangent_2 true)
    (`KismetArrayLibrary.Array_Add` (`self.meshes`) _returnvalue)))