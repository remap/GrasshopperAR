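; BP_VRController is the player controller for VR mode, handling startup, UI toggling and level switching.
; On BeginPlay it warns if the device is AR-capable; otherwise it binds the master UI delegate and streams in the base VR level.
; Number keys swap streamed game and lobby levels, unloading the previous one and teleporting the pawn to a player start.
; UI Toggle flips the mouse cursor and toggles master UI through the GameInstance.
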(event `Key|One`
  (params (Key :type "Key Structure"))
  (bind _gamelevel1 (`self.gameLevel1`))
  (:`Pressed`
    (`GameplayStatics.LoadStreamLevel` _gamelevel1 true true)
    (`GameplayStatics.UnloadStreamLevel` (`self.past level`))
    (`self.K2_SetActorLocation` (`self.K2_GetPawn`) (`self.K2_GetActorLocation` (`GameModeBase.K2_FindPlayerStart` (`GameplayStatics.GetGameMode`) null "")) false true)
    (set `self.past level` _gamelevel1)))

(event `Key|Zero`
  (params (Key :type "Key Structure"))
  (bind _gamelevel_lobby (`self.gameLevel_Lobby`))
  (:`Pressed`
    (`GameplayStatics.LoadStreamLevel` _gamelevel_lobby true true)
    (`GameplayStatics.UnloadStreamLevel` (`self.past level`))
    (`self.K2_SetActorLocation` (`self.K2_GetPawn`) (`self.K2_GetActorLocation` (`GameModeBase.K2_FindPlayerStart` (`GameplayStatics.GetGameMode`) null "")) false true)
    (set `self.past level` _gamelevel_lobby)))

(event `self.ReceiveBeginPlay`
  (`DDBlueprintLibrary.LogDebug` "VR PLAYER CONTROLLER BEGIN PLAY")
  (bind _returnvalue (`blueprintHelpers.isArCapableDevice`))
  (if _returnvalue
    (`self.On BeginPlay AR`)
    (else
      (`self.On BeginPlay VR`))))

(event `On BeginPlay AR`
  (`DDBlueprintLibrary.LogWarning` "VR PlayerController not supported in AR mode. How did this happen?"))

(event `On BeginPlay VR`
  (`|ExecutionSequence`
    (:`then_0`
      ;[1 0 0.672] VR Master UI Setup
      (add `self.OnToggleMasterUiDelegate` (delegate `On Toggle Master UI`)))
    (:`then_1`
      (`GameplayStatics.LoadStreamLevel` "M_BaseVR" true))))

(event `InputAction|UI Toggle`
  (params (Key :type "Key Structure"))
  ;[1 0 0.672] VR Master UI Setup
  (:`Pressed`
    (`self.OnToggleMasterUiDelegate`)
    (set `self.bShowMouseCursor` (not (`self.bShowMouseCursor`)))))

(event `On Toggle Master UI`
  ;[1 0 0.672] VR Master UI Setup
  (bind _asbp_game_instance (cast `/Game/Blueprints/BP_GameInstance` (`GameplayStatics.GetGameInstance`)))
  (`/Game/Blueprints/BP_GameInstance.Toggle Master UI` _asbp_game_instance (`GameplayStatics.GetPlayerController` 0)))

(fn `UserConstructionScript`)