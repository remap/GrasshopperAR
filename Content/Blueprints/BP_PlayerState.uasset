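; Player state Blueprint that tracks whether a player is active in the game.
; A server RPC logs the change and sets IsGameActive on the given player's state.
; Its RepNotify logs the player entering or leaving, then has BP_GameInstance run SelectiveRenderPlayersCheck to update local rendering of other players.
; An avatar-hidden flag also exists, but its RepNotify is empty and its setter is disconnected.
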(event `self.OnRepNotify_IsGameActive`
  (bind _returnvalue (`KismetTextLibrary.Conv_StringToText` (`self.GetPlayerName` self)))
  ;[0.03063 0.9155 1] Local: On Game Active State Changed
  (if (`self.isGameActive`)
    (`DDBlueprintLibrary.LogDebug` (`KismetTextLibrary.Conv_TextToString` (`|FormatText` "Player {name} entered the game" _returnvalue)))
    (else
      (`DDBlueprintLibrary.LogDebug` (`KismetTextLibrary.Conv_TextToString` (`|FormatText` "Player {name} left the game" _returnvalue)))))
  ;[1 1 1] Check local rendering of all other players
  (bind _asbp_game_instance (cast `/Game/Blueprints/BP_GameInstance` (`GameplayStatics.GetGameInstance`)))
  (`/Game/Blueprints/BP_GameInstance.Selective Render Players Check` _asbp_game_instance self))

(event `self.OnRepNotify_IsAvatarHidden`)

(event `RPC Server Set Player Active`
  (params (player :type "GHBasePlayerController Object Reference") (isActive :type Boolean))
  ;[0.6865 0.4272 1] Server: Set Player IsGameActive Flag
  (bind _returnvalue (`GHBasePlayerController.getPlayerState` player))
  (`DDBlueprintLibrary.LogDebug` (`KismetTextLibrary.Conv_TextToString` (`|FormatText` "Set player {playerName} active: {isActive}" (`KismetTextLibrary.Conv_StringToText` (`PlayerState.PlayerName` _returnvalue)) (`KismetTextLibrary.Conv_BoolToText` isActive))))
  (`self.SetIsGameActive` _returnvalue isActive))

(fn `UserConstructionScript`)