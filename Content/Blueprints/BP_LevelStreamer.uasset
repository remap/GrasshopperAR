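; Trigger volume actor that streams a configurable sublevel in and out as the player moves through it.
; When the player character begins overlapping the Box, it loads LevelToStream as visible with a blocking load; ending the overlap unloads it without blocking.
; Keys 1 and 2 manually trigger the same load and unload, independent of the volume.
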(event `Key|One`
  (params (Key :type "Key Structure"))
  (:`Pressed`
    (`GameplayStatics.LoadStreamLevel` (`self.LevelToStream`) true true)))

(event `Key|Two`
  (params (Key :type "Key Structure"))
  (:`Pressed`
    (`GameplayStatics.UnloadStreamLevel` (`self.LevelToStream`))))

(event `self.Box.OnComponentEndOverlap`
  (params (OverlappedComponent :type "PrimitiveComponent Object Reference") (OtherActor :type "Actor Object Reference") (OtherComp :type "PrimitiveComponent Object Reference") (OtherBodyIndex :type Integer))
  (if (== OtherActor (`GameplayStatics.GetPlayerCharacter` 0))
    (`GameplayStatics.UnloadStreamLevel` (`self.LevelToStream`))))

(event `self.Box.OnComponentBeginOverlap`
  (params (OverlappedComponent :type "PrimitiveComponent Object Reference") (OtherActor :type "Actor Object Reference") (OtherComp :type "PrimitiveComponent Object Reference") (OtherBodyIndex :type Integer) (bFromSweep :type Boolean) (SweepResult :type "HitResult Structure (by ref)"))
  (if (== OtherActor (`GameplayStatics.GetPlayerCharacter` 0))
    (`GameplayStatics.LoadStreamLevel` (`self.LevelToStream`) true true)))

(fn `UserConstructionScript`)