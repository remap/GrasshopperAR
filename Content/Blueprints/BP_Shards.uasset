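; BP_Shards is an actor with four shard meshes that share a textured material, apparently to display video.
; Construction creates one dynamic instance of MP_ShardMaterial, overwrites its texture parameter while looping through Texture, and assigns it to every shard.
; BeginPlay nests media player iteration inside media source iteration, repeatedly opening and playing sources on each player.
; All array lookups use the loop index plus one, skipping the first element and overrunning the last.
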(event `self.ReceiveBeginPlay`
  (`|ExecutionSequence`
    (:`then_0`
      (for (_ _array_index) (`self.mediaSource`)
        (for (_ _array_index_2) (`self.mediaPlayer`)
          (bind _output (`|GetArrayItem` (`self.mediaPlayer`) (+ _array_index_2 1)))
          (`MediaPlayer.OpenSource` _output (`|GetArrayItem` (`self.mediaSource`) (+ _array_index 1)))
          (`MediaPlayer.Play` _output))))))

(event `self.ReceiveTick`
  (params (DeltaSeconds :type "Float (single-precision)")))

(fn `UserConstructionScript`
  (bind _texture (`self.Texture`))
  (bind _returnvalue (`KismetMaterialLibrary.CreateDynamicMaterialInstance` "/Game/Movies/AMFN_2021_MediaPlayers/Scene4_MediaPlayers/MP_ShardMaterial.MP_ShardMaterial"))
  (for (_ _array_index) _texture
    (`MaterialInstanceDynamic.SetTextureParameterValue` _returnvalue (`self.TextureParameter`) (`|GetArrayItem` _texture (+ _array_index 1)))
    (`|ExecutionSequence`
      (:`then_0`
        (`PrimitiveComponent.SetMaterial` (`self.Shard_1`) 0 _returnvalue))
      (:`then_1`
        (`PrimitiveComponent.SetMaterial` (`self.Shard_2`) 0 _returnvalue))
      (:`then_2`
        (`PrimitiveComponent.SetMaterial` (`self.Shard_3`) 0 _returnvalue))
      (:`then_3`
        (`PrimitiveComponent.SetMaterial` (`self.Shard_4`) 0 _returnvalue)))))